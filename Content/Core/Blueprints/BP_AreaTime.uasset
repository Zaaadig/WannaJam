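; BP_AreaTime is a spherical zone that slows or accelerates what enters it, set by the Slow flag and Force.
; A timeline grows the sphere to SizeMultiplier on BeginPlay.
; On overlap, characters get movement and jump changes, plus an optional bumper launch, platforms get scaled Vitesse, BP_ParentObject gets MovementInside, and other actors get CustomTimeDilation.
; End overlap restores normal behavior, using ActorList to track affected characters.
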(event OnComponentBeginOverlap(Sphere)
  (params (OverlappedComponent :type Primitive%20Component%20Object%20Reference) (OtherActor :type Actor%20Object%20Reference) (OtherComp :type Primitive%20Component%20Object%20Reference) (OtherBodyIndex :type Integer) (bFromSweep :type Boolean) (SweepResult :type Hit%20Result%20Structure%20%28by%20ref%29))
  (bind _force (Variables|General|GetForce))
  (bind _output_get (Variables|Default|SetActorEntering OtherActor))
  (Variables|Default|SetSweepResult SweepResult)
  (if (.bSuccess (Utilities|Casting|CastToCharacter _output_get))
    (if (.bSuccess (Utilities|Casting|CastToBP_PlatMove_C (Variables|Default|GetActorEntering)))
      (Variables|Default|SetVitesse (Variables|/Game/Art/BP/platformes/BP_PlatMove_C.BP_PlatMove_C_C|GetVitesse (.AsBP%20Plat%20Move%20C (Utilities|Casting|CastToBP_PlatMove_C (Variables|Default|GetActorEntering)))))
      (if (Variables|General|GetbSlow?)
        (Variables|/Game/Art/BP/platformes/BP_PlatMove_C.BP_PlatMove_C_C|SetVitesse (.AsBP%20Plat%20Move%20C (Utilities|Casting|CastToBP_PlatMove_C (Variables|Default|GetActorEntering))) (* (Variables|/Game/Art/BP/platformes/BP_PlatMove_C.BP_PlatMove_C_C|GetVitesse (.AsBP%20Plat%20Move%20C (Utilities|Casting|CastToBP_PlatMove_C (Variables|Default|GetActorEntering)))) _force))
        (else
          (Variables|/Game/Art/BP/platformes/BP_PlatMove_C.BP_PlatMove_C_C|SetVitesse (.AsBP%20Plat%20Move%20C (Utilities|Casting|CastToBP_PlatMove_C (Variables|Default|GetActorEntering))) (/ (Variables|/Game/Art/BP/platformes/BP_PlatMove_C.BP_PlatMove_C_C|GetVitesse (.AsBP%20Plat%20Move%20C (Utilities|Casting|CastToBP_PlatMove_C (Variables|Default|GetActorEntering)))) _force))))
      (elif (Variables|General|GetbSlow?)
        (Variables|/Script/Engine.CharacterMovementComponent|SetMaxWalkSpeed (Variables|/Script/Engine.Character|GetCharacterMovement (.AsBP%20Character (Utilities|Casting|CastToBP_Character (Variables|Default|GetActorEntering)))) (/ (Variables|/Game/Core/Character/BP_Character.BP_Character_C|GetBaseSpeed (.AsBP%20Character (Utilities|Casting|CastToBP_Character (Variables|Default|GetActorEntering)))) (/ (Variables|General|GetForce) 1.5)))
        (Variables|/Script/Engine.CharacterMovementComponent|SetAirControl (Variables|/Script/Engine.Character|GetCharacterMovement (.AsBP%20Character (Utilities|Casting|CastToBP_Character (Variables|Default|GetActorEntering)))) 1.0)
        (Utilities|Array|Add (Variables|Default|GetActorList) (Variables|Default|GetActorEntering))
        (else
          (Variables|/Script/Engine.CharacterMovementComponent|SetJumpZVelocity (Variables|/Script/Engine.Character|GetCharacterMovement (.AsBP%20Character (Utilities|Casting|CastToBP_Character (Variables|Default|GetActorEntering)))) (Variables|Default|GetBoostedJumpForce))
          (Default|Accelerate (.AsBP%20Character (Utilities|Casting|CastToBP_Character (Variables|Default|GetActorEntering))))
          (Utilities|Array|Add (Variables|Default|GetActorList) (Variables|Default|GetActorEntering))
          (Variables|/Game/Core/Character/BP_Character.BP_Character_C|SetCurrentForceEffect (.AsBP%20Character (Utilities|Casting|CastToBP_Character (Variables|Default|GetActorEntering))) (Variables|General|GetForce))
          (Variables|/Game/Core/Character/BP_Character.BP_Character_C|SetBoostedJumpForce (.AsBP%20Character (Utilities|Casting|CastToBP_Character (Variables|Default|GetActorEntering))) (Variables|Default|GetBoostedJumpForce))
          (if (and (Variables|/Game/Core/Character/BP_Character.BP_Character_C|GetbJumping (.AsBP%20Character (Utilities|Casting|CastToBP_Character (Variables|Default|GetActorEntering)))) (Variables|Default|GetbIsBumper?))
            (Physics|AddImpulse (Variables|/Script/Engine.Character|GetCharacterMovement (.AsBP%20Character (Utilities|Casting|CastToBP_Character (Variables|Default|GetActorEntering)))) (* (+ (Math|Vector|Normalize (Transformation|GetActorForwardVector (.AsBP%20Character (Utilities|Casting|CastToBP_Character (Variables|Default|GetActorEntering))))) "0.000000,0.000000,1.000000") "1000.000000,1000.000000,1000.000000") true)))))
    (else
      (if (Variables|General|GetbSlow?)
        (Variables|Default|SetMovementInsideZone 5.0)
        (else
          (Variables|Default|SetMovementInsideZone 0.5)))
      (if (.bSuccess (Utilities|Casting|CastToBP_ParentObject (Variables|Default|GetActorEntering)))
        (Default|MovementInside (.AsBP%20Parent%20Object (Utilities|Casting|CastToBP_ParentObject (Variables|Default|GetActorEntering))) (Variables|Default|GetMovementInsideZone))
        (elif (Variables|General|GetbSlow?)
          (Variables|/Script/Engine.Actor|SetCustomTimeDilation (Variables|Default|GetActorEntering) (/ 1.0 (Variables|General|GetForce)))
          (else
            (Variables|/Script/Engine.Actor|SetCustomTimeDilation (Variables|Default|GetActorEntering) (Variables|General|GetForce))))))))

(event OnComponentEndOverlap(Sphere)
  (params (OverlappedComponent :type Primitive%20Component%20Object%20Reference) (OtherActor :type Actor%20Object%20Reference) (OtherComp :type Primitive%20Component%20Object%20Reference) (OtherBodyIndex :type Integer))
  (bind _output_get (Variables|Default|SetActorExiting OtherActor))
  (if (>= (Utilities|Array|FindItem (Variables|Default|GetActorList) _output_get) 0)
    (if (.bSuccess (Utilities|Casting|CastToBP_PlatMove_C (Variables|Default|GetActorExiting)))
      (Variables|/Game/Art/BP/platformes/BP_PlatMove_C.BP_PlatMove_C_C|SetVitesse (.AsBP%20Plat%20Move%20C (Utilities|Casting|CastToBP_PlatMove_C (Variables|Default|GetActorExiting))) (Variables|Default|GetVitesse))
      (elif (Variables|General|GetbSlow?)
        (Variables|/Script/Engine.CharacterMovementComponent|SetMaxWalkSpeed (Variables|/Script/Engine.Character|GetCharacterMovement (.AsBP%20Character (Utilities|Casting|CastToBP_Character (Utilities|Array|Get(acopy) (Variables|Default|GetActorList) (Utilities|Array|FindItem (Variables|Default|GetActorList) _output_get))))) (Variables|/Game/Core/Character/BP_Character.BP_Character_C|GetBaseSpeed (.AsBP%20Character (Utilities|Casting|CastToBP_Character (Utilities|Array|Get(acopy) (Variables|Default|GetActorList) (Utilities|Array|FindItem (Variables|Default|GetActorList) _output_get))))))
        (Utilities|Array|RemoveItem (Variables|Default|GetActorList) (Variables|Default|GetActorExiting))
        (Default|SlowtoNormal (.AsBP%20Character (Utilities|Casting|CastToBP_Character (Variables|Default|GetActorExiting))))
        (else
          (Variables|/Script/Engine.CharacterMovementComponent|SetJumpZVelocity (Variables|/Script/Engine.Character|GetCharacterMovement (.AsBP%20Character (Utilities|Casting|CastToBP_Character (Variables|Default|GetActorExiting)))) (Variables|Default|GetBaseJumpForce))
          (Utilities|Array|RemoveItem (Variables|Default|GetActorList) (Variables|Default|GetActorExiting))
          (Default|AcceleratetoNormal (.AsBP%20Character (Utilities|Casting|CastToBP_Character (Variables|Default|GetActorExiting)))))))
    (elif (.bSuccess (Utilities|Casting|CastToBP_ParentObject (Variables|Default|GetActorExiting)))
      (Default|StopMovementInsideZone (.AsBP%20Parent%20Object (Utilities|Casting|CastToBP_ParentObject (Variables|Default|GetActorExiting))))
      (Physics|SetSimulatePhysics (Variables|/Game/Core/Blueprints/BP_ParentObject.BP_ParentObject_C|GetStaticMesh (.AsBP%20Parent%20Object (Utilities|Casting|CastToBP_ParentObject (Variables|Default|GetActorExiting)))) true)
      (else
        (Variables|/Script/Engine.Actor|SetCustomTimeDilation (Variables|Default|GetActorExiting) 1.0)))))

(event EventBeginPlay
  (Components|Timeline|SetPlayRate (Variables|Default|GetTL_Start) (/ 1.0 0.1))
  (bind _alpha (Timeline|TL_Start PlayFromStart)
    (:Update
      (Transformation|SetWorldScale3D (Variables|Default|GetSphere) (Math|Vector|Lerp(Vector) "0, 0, 0" (* "1.000000,1.000000,1.000000" (Variables|General|GetSizeMultiplier)) _alpha)))))

(fn ConstructionScript
  (Transformation|SetWorldScale3D (Variables|Default|GetSphere) (* "1.000000,1.000000,1.000000" (Variables|General|GetSizeMultiplier)))
  (if (Variables|General|GetbShowSphere?)
    (Development|SetHiddeninGame (Variables|Default|GetSphere) false false)
    (else
      (Development|SetHiddeninGame (Variables|Default|GetSphere) true false))))