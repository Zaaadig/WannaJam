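; Parent actor for a physics object with configurable mesh and scale that can be moved in a controlled glide inside a zone.
; A looping timer samples the mesh location to track its travel direction.
; On zone movement, physics turns off and a timeline slides the mesh along a new straight spline in that direction over the given duration.
; When the timeline finishes or is stopped, physics resumes with an impulse along the stored direction.
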(event Custom|Code
  (Variables|Default|SetLastLoc (Variables|Default|GetCurrentLoc))
  (Variables|Default|SetCurrentLoc (Transformation|GetWorldLocation (Variables|Default|GetStaticMesh))))

(event Custom|MovementInside
  (params (MovementInsideZone :type Float%20%28double-precision%29))
  (Variables|Default|SetMovementInsideZoneDuration MovementInsideZone)
  (Variables|Default|SetStartLoc (Transformation|GetWorldLocation (Variables|Default|GetStaticMesh)))
  (bind _output_get (Variables|Default|SetCurrentDirection (- (Variables|Default|GetCurrentLoc) (Variables|Default|GetLastLoc))))
  (Variables|Default|SetEndLoc (+ (Variables|Default|GetStartLoc) (* (Math|Vector|Normalize _output_get) 1e+03)))
  (bind _returnvalue (AddComponent|AddSplineComponent false (Transformation|GetActorTransform self)))
  (Variables|Default|SetSplineComponent _returnvalue)
  (Utilities|Array|Clear (Variables|Default|GetPoints))
  (Utilities|Array|Add (Variables|Default|GetPoints) (Variables|Default|GetStartLoc))
  (Utilities|Array|Add (Variables|Default|GetPoints) (Variables|Default|GetEndLoc))
  (Spline|SetSplinePoints (Variables|Default|GetSplineComponent) (Variables|Default|GetPoints) "World" true)
  (Physics|SetSimulatePhysics (Variables|Default|GetStaticMesh) false)
  (Components|Timeline|SetPlayRate (Variables|Default|GetTL_MoveInsideZone) (/ 1.0 (Variables|Default|GetMovementInsideZoneDuration)))
  (bind _time (Timeline|TL_MoveInsideZone PlayFromStart)
    (:Update
      (Transformation|SetWorldLocation (Variables|Default|GetStaticMesh) (Spline|GetLocationatTime (Variables|Default|GetSplineComponent) _time "World" true) false false))
    (:Finished
      (Physics|SetSimulatePhysics (Variables|Default|GetStaticMesh) true)
      (Physics|AddImpulse (Variables|Default|GetStaticMesh) (* (Variables|Default|GetCurrentDirection) 1e+01) "None" false))))

(event Custom|StopMovementInsideZone
  (Utilities|FlowControl|Sequence
    (:then_0
      (bind _time (Timeline|TL_MoveInsideZone Stop)
        (:Update
          (Transformation|SetWorldLocation (Variables|Default|GetStaticMesh) (Spline|GetLocationatTime (Variables|Default|GetSplineComponent) _time "World" true) false false))
        (:Finished
          (Physics|SetSimulatePhysics (Variables|Default|GetStaticMesh) true)
          (Physics|AddImpulse (Variables|Default|GetStaticMesh) (* (Variables|Default|GetCurrentDirection) 1e+01) "None" false))))
    (:then_1
      (Utilities|FlowControl|DelayUntilNextTick)
      (Physics|SetSimulatePhysics (Variables|Default|GetStaticMesh) true)
      (Physics|AddImpulse (Variables|Default|GetStaticMesh) (* (Variables|Default|GetCurrentDirection) 1e+01) "None" true))))

(event EventBeginPlay
  (Variables|Default|SetCurrentLoc (Transformation|GetWorldLocation (Variables|Default|GetStaticMesh)))
  (Utilities|Time|SetTimerbyEvent (delegate Custom|Code) 0.1 true))

(fn ConstructionScript
  (Components|StaticMesh|SetStaticMesh (Variables|Default|GetStaticMesh) (Variables|Global|GetSM))
  (Transformation|SetWorldScale3D (Variables|Default|GetStaticMesh) (* "1.000000,1.000000,1.000000" (Variables|Global|GetScale))))