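; Trigger door that slides its mesh from its initial relative location to End.
; A character entering the main box plays the timeline lerp, with play rate scaled by AnimDuration.
; Overlapping the button box instead stores this door on BP_Character, presumably so the character can call PlayAnim.
; The construction script applies configurable meshes, trigger and button placement, and box scales.
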(event OnComponentBeginOverlap(Box)
  (params (OverlappedComponent :type Primitive%20Component%20Object%20Reference) (OtherActor :type Actor%20Object%20Reference) (OtherComp :type Primitive%20Component%20Object%20Reference) (OtherBodyIndex :type Integer) (bFromSweep :type Boolean) (SweepResult :type Hit%20Result%20Structure%20%28by%20ref%29))
  (Utilities|Casting|CastToBP_Character OtherActor)
  (CallFunction|PlayAnim))

(event OnComponentBeginOverlap(BoxButton)
  (params (OverlappedComponent :type Primitive%20Component%20Object%20Reference) (OtherActor :type Actor%20Object%20Reference) (OtherComp :type Primitive%20Component%20Object%20Reference) (OtherBodyIndex :type Integer) (bFromSweep :type Boolean) (SweepResult :type Hit%20Result%20Structure%20%28by%20ref%29))
  (bind _asbp_character (Utilities|Casting|CastToBP_Character OtherActor))
  (Variables|/Game/Core/Character/BP_Character.BP_Character_C|SetBP_TriggerDoor _asbp_character self))

(event Custom|PlayAnim
  (Components|Timeline|SetPlayRate (Variables|Default|GetTL_Anim) (/ 1.0 (Variables|Default|GetAnimDuration)))
  (bind _alpha (Timeline|TL_Anim PlayFromStart)
    (:Update
      (Transformation|SetRelativeLocation (Variables|Default|GetStaticMesh) (Math|Vector|Lerp(Vector) (Variables|Default|GetStart) (Variables|Default|GetEnd) _alpha) false false))))

(event EventBeginPlay)

(event Collision|EventActorBeginOverlap
  (params (OtherActor :type Actor%20Object%20Reference)))

(event EventTick
  (params (DeltaSeconds :type Float%20%28single-precision%29)))

(fn ConstructionScript
  (Components|StaticMesh|SetStaticMesh (Variables|Default|GetStaticMesh) (Variables|Default|GetSM_Door))
  (Components|StaticMesh|SetStaticMesh (Variables|Default|GetButton) (Variables|Default|GetSM_Button))
  (Variables|Default|SetStart (Variables|/Script/Engine.SceneComponent|GetRelativeLocation (Variables|Default|GetStaticMesh)))
  (Transformation|SetWorldLocation (Variables|Default|GetBox) (Variables|Default|GetTriggerLocation) false false)
  (Transformation|SetWorldScale3D (Variables|Default|GetBox) (Variables|Default|GetTriggerScale))
  (Transformation|SetWorldLocation (Variables|Default|GetButton) (Variables|Default|GetButtonLocation) false false)
  (Transformation|SetWorldScale3D (Variables|Default|GetBoxButton) (Variables|Default|GetTriggerButtonScale)))