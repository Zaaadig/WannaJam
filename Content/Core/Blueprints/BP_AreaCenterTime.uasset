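; BP_AreaCenterTime is a box trigger zone that drives a time dilation effect on BP_Character actors inside it.
; On overlap start it passes its own location to the character's StartAreaCenterTimer, leaving the effect logic to the character.
; On overlap end it clears the character's timer handle and restores normal CustomTimeDilation.
; The construction script sizes the box uniformly from a Scale variable.
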(event OnComponentBeginOverlap(Box)
  (params (OverlappedComponent :type Primitive%20Component%20Object%20Reference) (OtherActor :type Actor%20Object%20Reference) (OtherComp :type Primitive%20Component%20Object%20Reference) (OtherBodyIndex :type Integer) (bFromSweep :type Boolean) (SweepResult :type Hit%20Result%20Structure%20%28by%20ref%29))
  (bind _output_get (Variables|Default|SetActorEntering OtherActor))
  (if (.bSuccess (Utilities|Casting|CastToBP_Character _output_get))
    (Default|StartAreaCenterTimer (.AsBP%20Character (Utilities|Casting|CastToBP_Character _output_get)) (Transformation|GetActorLocation self))))

(event OnComponentEndOverlap(Box)
  (params (OverlappedComponent :type Primitive%20Component%20Object%20Reference) (OtherActor :type Actor%20Object%20Reference) (OtherComp :type Primitive%20Component%20Object%20Reference) (OtherBodyIndex :type Integer))
  (bind _output_get (Variables|Default|SetActorExit OtherActor))
  (if (.bSuccess (Utilities|Casting|CastToBP_Character _output_get))
    (Utilities|Time|ClearandInvalidateTimerbyHandle (Variables|/Game/Core/Character/BP_Character.BP_Character_C|GetTimerHandle (.AsBP%20Character (Utilities|Casting|CastToBP_Character _output_get))))
    (Variables|/Script/Engine.Actor|SetCustomTimeDilation (.AsBP%20Character (Utilities|Casting|CastToBP_Character _output_get)) 1.0)))

(event EventBeginPlay)

(event Collision|EventActorBeginOverlap
  (params (OtherActor :type Actor%20Object%20Reference)))

(event EventTick
  (params (DeltaSeconds :type Float%20%28single-precision%29)))

(fn ConstructionScript
  (Transformation|SetWorldScale3D (Variables|Default|GetBox) (* "1.000000,1.000000,1.000000" (Variables|Default|GetScale))))