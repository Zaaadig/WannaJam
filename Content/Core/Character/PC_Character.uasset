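; Player controller for a time-manipulation character, handling time control and bullet shooting.
; BeginPlay adds input mapping contexts and the crosshair widget.
; Held inputs slow or accelerate global time dilation, with acceleration also rescaling a destructible platform's destruct delay.
; Two shoot inputs launch slow or accelerate BP_Bullets by impulse from the pawn's RefBullet, gated by CanShoot, and destroy any existing SlowZoneCreated.
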(event Input|EnhancedActionEvents|EnhancedInputActionIA_SlowTime
  (params (ActionValue :type Boolean) (ElapsedSeconds :type Float%20%28double-precision%29) (TriggeredSeconds :type Float%20%28double-precision%29) (InputAction :type Input%20Action%20Object%20Reference :default "/Game/Core/Character/Inputs/IA_SlowTime.IA_SlowTime"))
  (:Triggered
    (Utilities|Time|SetGlobalTimeDilation (Variables|Default|GetSlowValue)))
  (:Completed
    (Utilities|Time|SetGlobalTimeDilation 1.0)))

(event Input|EnhancedActionEvents|EnhancedInputActionIA_AccelerateTime
  (params (ActionValue :type Boolean) (ElapsedSeconds :type Float%20%28double-precision%29) (TriggeredSeconds :type Float%20%28double-precision%29) (InputAction :type Input%20Action%20Object%20Reference :default "/Game/Core/Character/Inputs/IA_AccelerateTime.IA_AccelerateTime"))
  (:Triggered
    (Utilities|Time|SetGlobalTimeDilation (Variables|Default|GetAccelerateValue))
    (if (Utilities|IsValid (Variables|Default|GetDestroyPlatVar))
      (Variables|/Game/Art/BP/platformes/BP_destroyPatVar.BP_destroyPatVar_C|SetDestruct%20delay (Variables|Default|GetDestroyPlatVar) (* (Variables|Default|GetBaseDelay) (Variables|Default|GetAccelerateValue)))))
  (:Completed
    (Utilities|Time|SetGlobalTimeDilation 1.0)
    (if (Utilities|IsValid (Variables|Default|GetDestroyPlatVar))
      (Variables|/Game/Art/BP/platformes/BP_destroyPatVar.BP_destroyPatVar_C|SetDestruct%20delay (Variables|Default|GetDestroyPlatVar) (/ (Variables|Default|GetBaseDelay) (Variables|Default|GetAccelerateValue))))))

(event Input|EnhancedActionEvents|EnhancedInputActionIA_Shoot
  (params (ActionValue :type Boolean) (ElapsedSeconds :type Float%20%28double-precision%29) (TriggeredSeconds :type Float%20%28double-precision%29) (InputAction :type Input%20Action%20Object%20Reference :default "/Game/Core/Character/Inputs/IA_Shoot.IA_Shoot"))
  (bind _returnvalue (Pawn|GetControlledPawn))
  (bind _asbp_character (Utilities|Casting|CastToBP_Character _returnvalue))
  (bind _refbullet (Variables|/Game/Core/Character/BP_Character.BP_Character_C|GetRefBullet _asbp_character))
  (bind _returnvalue_2 (Math|Vector|GetForwardVector _refbullet))
  (:Started
    (if (Variables|Default|GetbCanShoot?)
      (bind _returnvalue_3 (Game|SpawnActorfromClass "/Game/Core/Character/BP_Bullet.BP_Bullet_C" (Transformation|GetWorldTransform (Variables|/Game/Core/Character/BP_Character.BP_Character_C|GetRefBullet (.AsBP%20Character (Utilities|Casting|CastToBP_Character (Pawn|GetControlledPawn))))) "AlwaysSpawn" "MultiplyWithRoot" 0 true (Variables|Default|GetBulletMaxDuration) 0))
      (bind _output_get (Variables|Default|SetCurrentBullet _returnvalue_3))
      (Variables|/Game/Core/Character/BP_Bullet.BP_Bullet_C|SetParent _output_get self)
      (Variables|Default|SetbCanShoot? false)
      (Development|PrintString (Utilities|String|ToString(Vector) _returnvalue_2))
      (Physics|AddImpulse (Variables|/Game/Core/Character/BP_Bullet.BP_Bullet_C|GetStaticMesh (Variables|Default|GetCurrentBullet)) (* (Math|Vector|Normalize _returnvalue_2) 7.5e+03) "None" true)
      (if (Utilities|IsValid (Variables|Default|GetSlowZoneCreated))
        (Actor|DestroyActor (Variables|Default|GetSlowZoneCreated))))))

(event Input|EnhancedActionEvents|EnhancedInputActionIA_ShootAccelerate
  (params (ActionValue :type Boolean) (ElapsedSeconds :type Float%20%28double-precision%29) (TriggeredSeconds :type Float%20%28double-precision%29) (InputAction :type Input%20Action%20Object%20Reference :default "/Game/Core/Character/Inputs/IA_ShootAccelerate.IA_ShootAccelerate"))
  (bind _returnvalue (Pawn|GetControlledPawn))
  (bind _asbp_character (Utilities|Casting|CastToBP_Character _returnvalue))
  (bind _refbullet (Variables|/Game/Core/Character/BP_Character.BP_Character_C|GetRefBullet _asbp_character))
  (bind _returnvalue_2 (Math|Vector|GetForwardVector _refbullet))
  (:Started
    (if (Variables|Default|GetbCanShoot?)
      (bind _returnvalue_3 (Game|SpawnActorfromClass "/Game/Core/Character/BP_Bullet.BP_Bullet_C" (Transformation|GetWorldTransform (Variables|/Game/Core/Character/BP_Character.BP_Character_C|GetRefBullet (.AsBP%20Character (Utilities|Casting|CastToBP_Character (Pawn|GetControlledPawn))))) "AlwaysSpawn" "MultiplyWithRoot" 0 false (Variables|Default|GetBulletMaxDuration) 0))
      (bind _output_get (Variables|Default|SetCurrentBullet _returnvalue_3))
      (Variables|/Game/Core/Character/BP_Bullet.BP_Bullet_C|SetParent _output_get self)
      (Variables|Default|SetbCanShoot? false)
      (Development|PrintString (Utilities|String|ToString(Vector) _returnvalue_2))
      (Physics|AddImpulse (Variables|/Game/Core/Character/BP_Bullet.BP_Bullet_C|GetStaticMesh (Variables|Default|GetCurrentBullet)) (* (Math|Vector|Normalize _returnvalue_2) 7.5e+03) "None" true)
      (if (Utilities|IsValid (Variables|Default|GetSlowZoneCreated))
        (Actor|DestroyActor (Variables|Default|GetSlowZoneCreated))))))

(event EventBeginPlay
  (Input|AddMappingContext (PlayerController|LocalPlayerSubsystems|GetEnhancedInputLocalPlayerSubsystem (Game|GetPlayerController 0)) "/Game/Core/Character/Inputs/IMC_Character.IMC_Character" 0 "(bIgnoreAllPressedKeysUntilRelease=True,bForceImmediately=False,bNotifyUserSettings=False)")
  (Input|AddMappingContext (PlayerController|LocalPlayerSubsystems|GetEnhancedInputLocalPlayerSubsystem (Game|GetPlayerController 0)) "/Game/Core/Character/Inputs/IMC_MouseLook.IMC_MouseLook" 0 "(bIgnoreAllPressedKeysUntilRelease=True,bForceImmediately=False,bNotifyUserSettings=False)")
  (bind _returnvalue (Actor|GetActorOfClass "/Game/Debug/BP_TestSpeed.BP_TestSpeed_C"))
  (Variables|Default|SetTestSpeed _returnvalue)
  (bind _returnvalue_2 (UserInterface|CreateWidget "/Game/Core/Character/WB_CrossHair.WB_CrossHair_C"))
  (UserInterface|Viewport|AddtoViewport _returnvalue_2 0))

(fn ConstructionScript)