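; Projectile that spawns a slow or speed BP_AreaTime zone at its impact point, ignoring hits on BP_Character.
; IsSlow picks the zone's force, and the new zone and re-enabled shot flag are written back to Parent.
; Speed zones flag bumper targets and attach to the hit actor, whereas the slow branch attaches the bullet itself before destroying it.
; A lifetime timeout re-enables both shot types and destroys the bullet.
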(event OnComponentHit(StaticMesh)
  (params (HitComponent :type Primitive%20Component%20Object%20Reference) (OtherActor :type Actor%20Object%20Reference) (OtherComp :type Primitive%20Component%20Object%20Reference) (NormalImpulse :type Vector :default "0, 0, 0") (Hit :type Hit%20Result%20Structure%20%28by%20ref%29))
  (bind _impactpoint (Collision|BreakHitResult Hit))
  (bind _parent (Variables|Default|GetParent))
  (bind _parent_2 (Variables|Default|GetParent))
  (bind _output_get (Variables|Default|SetHitActor OtherActor))
  (if (not (.bSuccess (Utilities|Casting|CastToBP_Character _output_get)))
    (if (Variables|Default|GetbIsSlow?)
      (bind _returnvalue (Game|SpawnActorfromClass "/Game/Core/Blueprints/BP_AreaTime.BP_AreaTime_C" (Math|Transform|MakeTransform _impactpoint "0, 0, 0" "1.000000,1.000000,1.000000") "AlwaysSpawn" "MultiplyWithRoot" 0 (Variables|Default|GetbIsSlow?) (Variables|Default|GetSlowForce) true (Variables|Default|GetSizeMultiplier) false 0))
      (if (Variables|Default|GetbIsSlow?)
        (Variables|/Game/Core/Character/PC_Character.PC_Character_C|SetSlowZoneCreated _parent_2 _returnvalue)
        (Variables|/Game/Core/Character/PC_Character.PC_Character_C|SetbCanShootSlow? _parent_2 true)
        (else
          (Variables|/Game/Core/Character/PC_Character.PC_Character_C|SetFastZoneCreated (Variables|Default|GetParent) _returnvalue)
          (Variables|/Game/Core/Character/PC_Character.PC_Character_C|SetbCanShootSpeed? _parent_2 true)))
      (Transformation|AttachActorToActor (Variables|Default|GetHitActor) "None" "KeepWorld" "KeepWorld" "KeepWorld" true)
      (Actor|DestroyActor)
      (else
        (bind _returnvalue_2 (Game|SpawnActorfromClass "/Game/Core/Blueprints/BP_AreaTime.BP_AreaTime_C" (Math|Transform|MakeTransform _impactpoint "0, 0, 0" "1.000000,1.000000,1.000000") "AlwaysSpawn" "MultiplyWithRoot" 0 (Variables|Default|GetbIsSlow?) (Variables|Default|GetFastForce) true (Variables|Default|GetSizeMultiplier) (.bSuccess (Utilities|Casting|CastToBP_TargetBumper (Variables|Default|GetHitActor))) 0))
        (if (Variables|Default|GetbIsSlow?)
          (Variables|/Game/Core/Character/PC_Character.PC_Character_C|SetSlowZoneCreated _parent _returnvalue_2)
          (Variables|/Game/Core/Character/PC_Character.PC_Character_C|SetbCanShootSlow? _parent true)
          (else
            (Variables|/Game/Core/Character/PC_Character.PC_Character_C|SetFastZoneCreated (Variables|Default|GetParent) _returnvalue_2)
            (Variables|/Game/Core/Character/PC_Character.PC_Character_C|SetbCanShootSpeed? _parent true)))
        (Transformation|AttachActorToActor _returnvalue_2 (Variables|Default|GetHitActor) "None" "KeepWorld" "KeepWorld" "KeepWorld" true)
        (Actor|DestroyActor)))))

(event EventBeginPlay
  (Utilities|FlowControl|Delay (Variables|Default|GetBulletMaxDuration))
  (Variables|/Game/Core/Character/PC_Character.PC_Character_C|SetbCanShootSpeed? (Variables|Default|GetParent) true)
  (Variables|/Game/Core/Character/PC_Character.PC_Character_C|SetbCanShootSlow? (Variables|Default|GetParent) true)
  (Actor|DestroyActor))

(fn ConstructionScript)