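; BP_FLOOR is an environment Blueprint that builds a tiled floor from a chosen static mesh.
; The construction script fills an instanced static mesh component with a local-space grid, spacing tiles by the mesh's bounding box.
; NmbrCubesY sets the count along Y, while NmbrCubesZ, despite its name, sets the count along X.
; A vertical-stacking branch keyed on IsHorizontal is disconnected, and the event graph is empty.
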(event EventBeginPlay)

(event Collision|EventActorBeginOverlap
  (params (OtherActor :type Actor%20Object%20Reference)))

(event EventTick
  (params (DeltaSeconds :type Float%20%28single-precision%29)))

(fn ConstructionScript
  (bind _sm (Variables|Default|GetSM))
  (bind _sm_2 (Variables|Default|GetSM))
  (bind _returnvalue (StaticMesh|GetBoundingBox _sm))
  (bind _returnvalue_2 (StaticMesh|GetBoundingBox _sm_2))
  (Components|StaticMesh|SetStaticMesh (Variables|Default|GetInstancedStaticMesh) (Variables|Default|GetSM))
  (for _index (range 0 (- (Variables|Default|GetNmbr_Cubes_Y) 1))
    (for _index_2 (range 0 (- (Variables|Default|GetNmbr_Cubes_Z) 1))
      (Components|InstancedStaticMesh|AddInstance (Variables|Default|GetInstancedStaticMesh) (Math|Transform|MakeTransform (Math|Vector|MakeVector (* _index_2 (.x (- (.max _returnvalue) (.min _returnvalue)))) (* _index (.y (- (.max _returnvalue_2) (.min _returnvalue_2)))) 0.0)) false))))