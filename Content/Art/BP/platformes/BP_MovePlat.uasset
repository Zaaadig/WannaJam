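; BP_MovePlat is a moving platform that carries the player character.
; The construction script feeds two relative positions, Loc1 and Loc2, to an InterpToMovement component as control points.
; On actor overlap, it attaches any BP_Character to itself with keep-world rules and prints a debug message; the graph has no matching detach.
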(event EventBeginPlay)

(event Collision|EventActorBeginOverlap
  (params (OtherActor :type Actor%20Object%20Reference))
  (bind (_asbp_character _bsuccess) (Utilities|Casting|CastToBP_Character OtherActor))
  (if _bsuccess
    (Transformation|AttachActorToActor _asbp_character self "None" "KeepWorld" "KeepWorld" "KeepWorld" true)
    (Development|PrintString "Hello")))

(fn ConstructionScript
  (Class|InterptoMovementComponent|AddControlPointPosition (Variables|Default|GetInterpToMovement) (Variables|Default|GetLoc1) true)
  (Class|InterptoMovementComponent|AddControlPointPosition (Variables|Default|GetInterpToMovement) (Variables|Default|GetLoc2) true))