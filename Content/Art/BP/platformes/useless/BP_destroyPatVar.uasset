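; Moving platform that destroys itself a set delay after the player character touches it.
; The construction script feeds two relative points and a duration to InterpToMovement.
; Box overlap registers the platform and its delay on PC_Character, then starts a looping timer.
; Each tick of that timer adds 0.1 to a counter until it reaches DestructDelay and the actor is destroyed.
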(event OnComponentBeginOverlap(Box)
  (params (OverlappedComponent :type Primitive%20Component%20Object%20Reference) (OtherActor :type Actor%20Object%20Reference) (OtherComp :type Primitive%20Component%20Object%20Reference) (OtherBodyIndex :type Integer) (bFromSweep :type Boolean) (SweepResult :type Hit%20Result%20Structure%20%28by%20ref%29))
  (bind _returnvalue (Game|GetPlayerController 0))
  (bind _aspc_character (Utilities|Casting|CastToPC_Character _returnvalue))
  (Utilities|Casting|CastToBP_Character OtherActor)
  (Variables|/Game/Core/Character/PC_Character.PC_Character_C|SetDestroyPlatVar _aspc_character self)
  (Variables|/Game/Core/Character/PC_Character.PC_Character_C|SetBaseDelay _aspc_character (Variables|Default|GetDestruct%20delay))
  (bind _returnvalue_2 (Utilities|Time|SetTimerbyEvent (delegate Custom|DelayDestruct) (Variables|Default|GetTime) true)))

(event Custom|DelayDestruct
  (bind _output_get (Variables|Default|SetDelayCount (+ (Variables|Default|GetDelayCount) 0.1)))
  (if (>= _output_get (Variables|Default|GetDestruct%20delay))
    (Utilities|Time|ClearandInvalidateTimerbyHandle (stale OnComponentBeginOverlap(Box) _returnvalue_2))
    (Actor|DestroyActor)))

(event EventBeginPlay)

(event Collision|EventActorBeginOverlap
  (params (OtherActor :type Actor%20Object%20Reference)))

(event EventTick
  (params (DeltaSeconds :type Float%20%28single-precision%29)))

(fn ConstructionScript
  (Class|InterptoMovementComponent|AddControlPointPosition (Variables|Default|GetInterpToMovement) (Variables|Default|GetLoc1) true)
  (Class|InterptoMovementComponent|AddControlPointPosition (Variables|Default|GetInterpToMovement) (Variables|Default|GetLoc2) true)
  (Variables|/Script/Engine.InterpToMovementComponent|SetDuration (Variables|Default|GetInterpToMovement) (Variables|Default|GetDuration)))