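; Parent platform Blueprint that can move between two points or be destroyed when the character touches it, depending on its flags.
; With Move set, BeginPlay adds two relative control points and a duration to InterpToMovement.
; With Destroy set, character overlap passes itself and its delay to PC_Character, then destroys the platform immediately.
; The delay timer is cleared as soon as it is set, and its threshold check does nothing.
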(event OnComponentBeginOverlap(Box)
  (params (OverlappedComponent :type Primitive%20Component%20Object%20Reference) (OtherActor :type Actor%20Object%20Reference) (OtherComp :type Primitive%20Component%20Object%20Reference) (OtherBodyIndex :type Integer) (bFromSweep :type Boolean) (SweepResult :type Hit%20Result%20Structure%20%28by%20ref%29))
  (bind _returnvalue (Game|GetPlayerController 0))
  (bind _aspc_character (Utilities|Casting|CastToPC_Character _returnvalue))
  (if (Variables|Destroyable|GetDestroy%20?)
    (Development|PrintString "Hello")
    (Utilities|Casting|CastToBP_Character OtherActor)
    (Variables|/Game/Core/Character/PC_Character.PC_Character_C|SetBP_PlatParent _aspc_character self)
    (Variables|/Game/Core/Character/PC_Character.PC_Character_C|SetBaseDelay _aspc_character (Variables|Destroyable|GetDestrucDelay))
    (bind _returnvalue_2 (Utilities|Time|SetTimerbyEvent (delegate Custom|DelayDestruct) (Variables|Destroyable|GetTime) true))
    (Utilities|Time|ClearandInvalidateTimerbyHandle _returnvalue_2)
    (Actor|DestroyActor)
    (else
      (Development|PrintString "baaaaaa"))))

(event Custom|DelayDestruct
  (bind _output_get (Variables|Destroyable|SetDelayCount (+ (Variables|Destroyable|GetDelayCount) 0.1)))
  (if (>= _output_get (Variables|Destroyable|GetDestrucDelay))
    _))

(event Custom|Move
  (bind _interptomovement (Variables|Default|GetInterpToMovement))
  (Class|InterptoMovementComponent|AddControlPointPosition (Variables|Default|GetInterpToMovement) (Variables|Moving|GetLoc1) true)
  (Class|InterptoMovementComponent|AddControlPointPosition _interptomovement (Variables|Moving|GetLoc2) true)
  (Variables|/Script/Engine.InterpToMovementComponent|SetDuration _interptomovement (Variables|Moving|GetVitesse))
  (Development|PrintString (Utilities|String|ToString(Vector) (Transformation|GetActorLocation))))

(event EventBeginPlay
  (if (Variables|Moving|GetMove?)
    (CallFunction|Move)))

(event Collision|EventActorBeginOverlap
  (params (OtherActor :type Actor%20Object%20Reference)))

(event EventTick
  (params (DeltaSeconds :type Float%20%28single-precision%29)))

(fn ConstructionScript)