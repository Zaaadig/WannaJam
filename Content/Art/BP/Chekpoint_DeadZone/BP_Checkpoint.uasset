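; BP_Checkpoint is a checkpoint actor that records the player's respawn progress and can also end the game.
; When BP_Character enters its Box, it stores itself as GM_Game's LastCheckpoint, sets IsFirstChecked and switches on its PointLight, which starts dark.
; If flagged IsLastCheckpoint, it also shows the credits widget and mouse cursor and disables the character's movement.
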(event OnComponentBeginOverlap(Box)
  (params (OverlappedComponent :type Primitive%20Component%20Object%20Reference) (OtherActor :type Actor%20Object%20Reference) (OtherComp :type Primitive%20Component%20Object%20Reference) (OtherBodyIndex :type Integer) (bFromSweep :type Boolean) (SweepResult :type Hit%20Result%20Structure%20%28by%20ref%29))
  (bind _returnvalue (Game|GetPlayerController 0))
  (bind _asbp_character (Utilities|Casting|CastToBP_Character OtherActor))
  (bind _asgm_game (Utilities|Casting|CastToGM_Game (Game|GetGameMode)))
  (Variables|/Game/Core/GM_Game.GM_Game_C|SetLast%20checkpoint _asgm_game self)
  (Variables|/Game/Core/GM_Game.GM_Game_C|SetIsFirstChecked? _asgm_game true)
  (Rendering|Components|Light|SetIntensity (Variables|Default|GetPointLight) 18513.828125)
  (if (Variables|Default|Getis%20last%20checkpoint%20?)
    (bind _returnvalue_2 (UserInterface|CreateWidget "/Game/Widgets/WBP_Credits.WBP_Credits_C" _returnvalue))
    (UserInterface|Viewport|AddtoViewport _returnvalue_2 0)
    (Variables|/Script/Engine.PlayerController|SetbShowMouseCursor _returnvalue true)
    (Pawn|Components|CharacterMovement|DisableMovement (Variables|/Script/Engine.Character|GetCharacterMovement _asbp_character))))

(event EventBeginPlay
  (Rendering|Components|Light|SetIntensity (Variables|Default|GetPointLight) 0.0))

(event Collision|EventActorBeginOverlap
  (params (OtherActor :type Actor%20Object%20Reference)))

(event EventTick
  (params (DeltaSeconds :type Float%20%28single-precision%29)))

(fn ConstructionScript)