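; BP_Ventilo_ZAxis is a fan volume that pushes characters and other actors upward along Z.
; Capsule overlaps maintain the AffectedActors list, and entering switches a BP_Character to Falling.
; Each Tick relaunches characters below MaxUpVelocity by Force, overriding all axes, so horizontal velocity is zeroed.
; Other actors take the AddForce path, with acceleration change enabled when they have a StaticMeshComponent.
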(event OnComponentBeginOverlap(Capsule)
  (params (OverlappedComponent :type Primitive%20Component%20Object%20Reference) (OtherActor :type Actor%20Object%20Reference) (OtherComp :type Primitive%20Component%20Object%20Reference) (OtherBodyIndex :type Integer) (bFromSweep :type Boolean) (SweepResult :type Hit%20Result%20Structure%20%28by%20ref%29))
  (Utilities|Array|AddUnique (Variables|Default|GetAffectedActors) OtherActor)
  (bind _asbp_character (Utilities|Casting|CastToBP_Character OtherActor))
  (Pawn|Components|CharacterMovement|SetMovementMode (Variables|/Script/Engine.Character|GetCharacterMovement _asbp_character) "MOVE_Falling" 0))

(event OnComponentEndOverlap(Capsule)
  (params (OverlappedComponent :type Primitive%20Component%20Object%20Reference) (OtherActor :type Actor%20Object%20Reference) (OtherComp :type Primitive%20Component%20Object%20Reference) (OtherBodyIndex :type Integer))
  (Utilities|Array|RemoveItem (Variables|Default|GetAffectedActors) OtherActor))

(event EventBeginPlay)

(event Collision|EventActorBeginOverlap
  (params (OtherActor :type Actor%20Object%20Reference)))

(event EventTick
  (params (DeltaSeconds :type Float%20%28single-precision%29))
  (for _array_element (Variables|Default|GetAffectedActors)
    (bind _asbp_character (Utilities|Casting|CastToBP_Character _array_element)
      (:then
        (if (< (.z (Transformation|GetVelocity _asbp_character)) (Variables|Default|GetMaxUpVelocity))
          (Character|LaunchCharacter _asbp_character (Math|Vector|MakeVector 0.0 0.0 (Variables|Default|GetForce)) true true)))
      (:CastFailed
        (Physics|AddForce :Force (Math|Vector|MakeVector 0.0 0.0 (Variables|Default|GetForce)) :bAccelChange (Utilities|IsValid (Actor|GetComponentbyClass _array_element "/Script/Engine.StaticMeshComponent")))))))

(fn ConstructionScript)